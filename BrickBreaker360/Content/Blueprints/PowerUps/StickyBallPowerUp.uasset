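; Sticky ball power-up for a brick breaker game that makes the ball sticky when activated.
; Activation calls the parent logic, finds a BrickBreaker360Ball_BP actor by class, caches it and sets its IsSticky flag.
; Tick calls UpdatePowerUpTimer only while that cached ball is valid and attached, so the timer is not updated from here while the ball is detached.
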(event EventBeginPlay)

(event Collision|EventActorBeginOverlap
  (params (OtherActor :type Actor%20Object%20Reference)))

(event EventTick
  (params (DeltaSeconds :type Float%20%28single-precision%29))
  (bind _ball (Variables|Default|GetBall))
  (if (Utilities|IsValid _ball)
    (if (Variables|/Script/BrickBreaker360.BrickBreaker360Ball|GetIsAttached _ball)
      (Class|PowerUpBase|UpdatePowerUpTimer))))

(event EventActivatePowerUp
  (|CallParentFunction)
  (bind _returnvalue (Actor|GetActorOfClass "/Game/Blueprints/BrickBreaker360Ball_BP.BrickBreaker360Ball_BP_C"))
  (bind _output_get (Variables|Default|SetBall _returnvalue))
  (if (Utilities|IsValid _returnvalue)
    (Variables|/Script/BrickBreaker360.BrickBreaker360Ball|SetIsSticky _output_get true)))

(fn ConstructionScript)